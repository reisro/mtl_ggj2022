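; CubeBP is an actor that moves its static mesh from its starting location to the location of a referenced TargetPoint.
; On BeginPlay it caches both locations and plays a timeline.
; Each timeline update passes its Alpha to MoveTo, which lerps between the two points and sets the mesh's world location without sweeping, so collisions do not block the movement.
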(event `self.ReceiveBeginPlay`
  (set `self.Start` (`self.K2_GetActorLocation`))
  (set `self.End` (`self.K2_GetActorLocation` (`self.TargetPoint`)))
  (bind (_direction _alpha) (`Timeline|Timeline_0`)
    (:`Update`
      (`self.MoveTo` _alpha))))

(fn `MoveTo`
  (params (Alpha :type "Float (double-precision)"))
  (`SceneComponent.K2_SetWorldLocation` (`self.StaticMeshComponent`) (`KismetMathLibrary.VLerp` (`self.Start`) (`self.End`) Alpha) false false))

(fn `UserConstructionScript`)