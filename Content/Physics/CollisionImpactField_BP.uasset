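; Field system actor that applies an impact to physics objects, such as destructible geometry, when play begins.
; A sphere component sets location and radius for the dynamic state field and the falloff that scales radial velocity.
; Uniform and random vectors multiply into angular torque, while the external strain field has no node connected.
; A two-second delay leads nowhere, and DestroyActor is unwired, so the actor never destroys itself.
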(event `self.ReceiveBeginPlay`
  (bind _sphere (`self.Sphere`))
  (bind _sphere_2 (`self.Sphere`))
  (`|ExecutionSequence`
    (:`then_0`
      (`FieldSystemComponent.ApplyPhysicsField` (`self.FieldSystemComponent`) true "Field_DynamicState" null (`RadialFalloff.SetRadialFalloff` (`self.RadialFalloff`) (`self.StrainMagnitude`) 0.0 1.0 0.0 (* (.x (`SceneComponent.K2_GetComponentScale` _sphere_2)) 50.0) (`SceneComponent.K2_GetComponentLocation` _sphere_2) "Field_FallOff_None"))
      (`FieldSystemComponent.ApplyPhysicsField` (`self.FieldSystemComponent`) true "Field_ExternalClusterStrain" null null)
      (`FieldSystemComponent.ApplyPhysicsField` (`self.FieldSystemComponent`) true "Field_LinearVelocity" null (`OperatorField.SetOperatorField` (`self.OperatorField`) 1.0 (`RadialFalloff.SetRadialFalloff` (`self.RadialFalloff`) (`self.StrainMagnitude`) 0.0 1.0 0.0 (* (.x (`SceneComponent.K2_GetComponentScale` _sphere)) 50.0) (`SceneComponent.K2_GetComponentLocation` _sphere) "Field_Falloff_Linear") (`RadialVector.SetRadialVector` (`self.RadialVector`) (`self.ForceMagnitude`) (`SceneComponent.K2_GetComponentLocation` (`self.FieldSystemComponent`))) "Field_Multiply"))
      (`FieldSystemComponent.ApplyPhysicsField` (`self.FieldSystemComponent`) true "Field_AngularTorque" null (`OperatorField.SetOperatorField` (`self.OperatorField`) 1.0 (`UniformVector.SetUniformVector` (`self.UniformVector`) 1.0 (4.0 0.0 10.0)) (`RandomVector.SetRandomVector` (`self.RandomVector`) 100000.0) "Field_Multiply")))
    (:`then_1`
      (`KismetSystemLibrary.Delay` 2.0))))

(fn `UserConstructionScript`)