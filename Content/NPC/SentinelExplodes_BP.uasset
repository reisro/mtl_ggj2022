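; Sentinel NPC character that sets off an impact field on spawn and explodes on contact with the player.
; BeginPlay waits briefly, then spawns a CollisionImpactField_BP just above the actor's location.
; A capsule hit from an actor tagged Player spawns a spark explosion emitter and destroys the Sentinel.
; A Fly function zeroes gravity but is not called within this Blueprint, and both events print debug text.
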(event `self.ReceiveBeginPlay`
  (`KismetSystemLibrary.PrintString` "Boom")
  (`KismetSystemLibrary.Delay` 0.2)
  (`|SpawnActorFromClass` "/Game/Physics/CollisionImpactField_BP.CollisionImpactField_BP_C" (`KismetMathLibrary.Conv_VectorToTransform` (`KismetMathLibrary.MakeVector` (.x (`self.K2_GetActorLocation`)) (.y (`self.K2_GetActorLocation`)) (+ (.z (`self.K2_GetActorLocation`)) 80.0))) "Undefined" "OverrideRootScale" null 250.0 null))

(event `self.CapsuleComponent.OnComponentBeginOverlap`
  (params (OverlappedComponent :type "PrimitiveComponent Object Reference") (OtherActor :type "Actor Object Reference") (OtherComp :type "PrimitiveComponent Object Reference") (OtherBodyIndex :type Integer) (bFromSweep :type Boolean) (SweepResult :type "HitResult Structure (by ref)")))

(event `self.CapsuleComponent.OnComponentHit`
  (params (HitComponent :type "PrimitiveComponent Object Reference") (OtherActor :type "Actor Object Reference") (OtherComp :type "PrimitiveComponent Object Reference") (NormalImpulse :type "Vector Structure") (Hit :type "HitResult Structure (by ref)"))
  (if (`self.ActorHasTag` OtherActor "Player")
    (`KismetSystemLibrary.PrintString` "Boom")
    (`GameplayStatics.SpawnEmitterAtLocation` "/Game/GameJamKit/Effects/Explosions/P_explosionSpark.P_explosionSpark" (`self.K2_GetActorLocation`))
    (`self.K2_DestroyActor`)))

(fn `Fly`
  (set `CharacterMovementComponent.GravityScale` 0.0 (`self.CharacterMovement`)))

(fn `UserConstructionScript`)