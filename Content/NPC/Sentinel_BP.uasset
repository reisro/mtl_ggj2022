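; Flying Sentinel NPC that patrols or runs AI, and explodes when it collides with the player.
; Leaders loop through a Destination actor list, lerping position with a restarting timeline; others run the Sentinel_BT behavior tree.
; A short forward line trace on Tick only prints when it detects the player.
; Gravity is disabled for flight, and a quantum-captured event relays to CallOnQuantumCaptured.
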(event `self.ReceiveBeginPlay`
  (`self.Fly`)
  (if (`self.isLeader`)
    (set `self.CurrentPosition` (`self.K2_GetActorLocation`))
    (`self.OnPatrol`)
    (`self.UpdateDestination`)
    (else
      (`AIController.RunBehaviorTree` (`AIBlueprintHelperLibrary.GetAIController` self) "/Game/NPC/AI/Sentinel_BT.Sentinel_BT"))))

(event `self.ReceiveTick`
  (params (DeltaSeconds :type "Float (single-precision)"))
  (bind (_outhit _returnvalue) (`KismetSystemLibrary.LineTraceSingle` :`Start` (`self.K2_GetActorLocation`) :`End` (+ (`self.K2_GetActorLocation`) (* (`SceneComponent.GetForwardVector` (`self.Body`)) 50.0)) :`TraceChannel` "TraceTypeQuery1" :`DrawDebugType` "ForDuration" :`DrawTime` 1.0))
  (if _returnvalue
    (bind (_bblockinghit _binitialoverlap _time _distance _location _impactpoint _normal _impactnormal _physmat _hitactor) (`GameplayStatics.BreakHitResult` _outhit))
    (if (`KismetSystemLibrary.IsValid` _hitactor)
      (if (`self.ActorHasTag` _hitactor "Player")
        (`KismetSystemLibrary.PrintString` "Detected enemy")))))

(event `OnPatrol`
  (bind (_direction _alpha) (`Timeline|OnPatrolTimeline`)
    (:`Update`
      (`self.MoveTo` _alpha))
    (:`Finished`
      (`self.OnReachedDestination`))))

(event `OnEnemyDetected`)

(event `OnReachedDestination`
  (`self.UpdateDestination`)
  (set `self.CurrentPosition` (`self.K2_GetActorLocation`))
  (`TimelineComponent.SetNewTime` (`self.OnPatrolTimeline`) 0.0)
  (`self.OnPatrol`))

(event `OnQuantumCapturedEvent`
  (`self.OnQuantumCaptured`))

(event `self.CapsuleComponent.OnComponentHit`
  (params (HitComponent :type "PrimitiveComponent Object Reference") (OtherActor :type "Actor Object Reference") (OtherComp :type "PrimitiveComponent Object Reference") (NormalImpulse :type "Vector Structure") (Hit :type "HitResult Structure (by ref)"))
  (bind (_bblockinghit _binitialoverlap _time _distance _location) (`GameplayStatics.BreakHitResult` Hit))
  (if (`self.ActorHasTag` OtherActor "Player")
    (`/Engine/EditorBlueprintResources/StandardMacros.DoOnce` false
      (:`Completed`
        (`GameplayStatics.SpawnEmitterAtLocation` "/Game/Effects/Explosions/P_explosionSpark.P_explosionSpark" _location)
        (`GameplayStatics.PlaySoundAtLocation` "/Game/Quantum_Audio_Files/Enemy/Enemy_Destroyed.Enemy_Destroyed" _location (struct) 1.0 1.0 0.0 null null null)
        (`self.K2_DestroyActor`)))))

(fn `Fly`
  (set `CharacterMovementComponent.GravityScale` 0.0 (`self.CharacterMovement`)))

(fn `MoveTo`
  (params (Alpha :type "Float (double-precision)"))
  (`self.K2_SetActorLocation` (`KismetMathLibrary.VLerp` (`self.CurrentPosition`) (`self.NextPosition`) Alpha)))

(fn `UpdateDestination`
  (returns (Ended :type Boolean))
  (bind _destination (`self.Destination`))
  (bind _result (`/Engine/EditorBlueprintResources/StandardMacros.IncrementInt` (`self.destID`))
    (:`  `
      (if (<= _result (- (`KismetArrayLibrary.Array_Length` _destination) 1))
        (set `self.NextPosition` (`self.K2_GetActorLocation` (`|GetArrayItem` _destination _result)))
        (return false)
        (else
          (set `self.destID` -1)
          (return true))))))

(fn `UserConstructionScript`)